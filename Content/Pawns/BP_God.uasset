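; BP_God is a player pawn that directs a multi-legged spider pawn to points the player clicks in the world.
; On BeginPlay it caches the first MultiLeggedPawn and NavVolume found in the level.
; Left click traces along the camera's view, offsets the hit along its surface normal, then asks the NavVolume for a path using the spider's preference and hands it to the spider.
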(event EventBeginPlay
  (bind _returnvalue (Actor|GetActorOfClass "/Script/Entomon.MultiLeggedPawn"))
  (Variables|Default|SetSpider _returnvalue)
  (bind _returnvalue_2 (Actor|GetActorOfClass "/Script/Entomon.NavVolume"))
  (Variables|Default|SetNavigation _returnvalue_2))

(event Collision|EventActorBeginOverlap
  (params (OtherActor :type Actor%20Object%20Reference)))

(event EventTick
  (params (DeltaSeconds :type Float%20%28single-precision%29)))

(event Input|MouseEvents|LeftMouseButton
  (params (Key :type Key%20Structure :default "None"))
  (bind _returnvalue (Game|GetPlayerCameraManager 0))
  (bind _spider (Variables|Default|GetSpider))
  (bind _returnvalue_2 (Camera|GetCameraLocation _returnvalue))
  (:Pressed
    (bind (_outhit _returnvalue_3) (Collision|LineTraceByChannel _returnvalue_2 (+ _returnvalue_2 (* (Math|Vector|GetForwardVector (Variables|/Script/Engine.PlayerCameraManager|GetTransformComponent _returnvalue)) (Variables|Default|GetCast%20Distance))) "TraceTypeQuery1" false 0 "ForDuration" true "(R=1.000000,G=0.000000,B=0.000000,A=1.000000)" "(R=0.000000,G=1.000000,B=0.000000,A=1.000000)" 2.0))
    (if _returnvalue_3
      (bind _returnvalue_4 (Class|NavVolume|FindPath (Variables|Default|GetNavigation) (Transformation|GetActorLocation _spider) (+ (.Location (Collision|BreakHitResult _outhit)) (* (.Normal (Collision|BreakHitResult _outhit)) 65.0)) (Variables|/Script/Entomon.MultiLeggedPawn|GetPathPreference _spider)))
      (Class|MultiLeggedPawn|SetPath _spider _returnvalue_4))))

(fn ConstructionScript)